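; BP_Controller is a controller Blueprint that turns player input into actions on player 0's pawn and character.
; Move axes add movement input, forward along the yaw-only control rotation and sideways along its own actor right vector.
; Turn and look axes feed yaw and pitch input, and Jump calls the character's jump.
; Attack casts the character to BP_Player and calls Fire, printing a message if the cast fails.
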(event Input|ActionEvents|InputActionJump
  (params (Key :type Key%20Structure))
  (:Pressed
    (Character|Jump (Game|GetPlayerCharacter 0))))

(event Input|ActionEvents|InputActionAttack
  (params (Key :type Key%20Structure))
  (:Pressed
    (bind _asbp_player (Utilities|Casting|CastToBP_Player (Game|GetPlayerCharacter 0))
      (:then
        (Default|Fire _asbp_player))
      (:CastFailed
        (Development|PrintString "캐스팅 실패")))))

(event Input|AxisEvents|InputAxisMoveForward
  (params (AxisValue :type Float%20%28single-precision%29))
  (Pawn|Input|AddMovementInput (Game|Player|GetPlayerPawn 0) (Math|Vector|GetForwardVector (Math|Rotator|MakeRotator 0.0 0.0 (.yaw (Pawn|GetControlRotation :!class /Script/Engine.Controller)))) AxisValue false))

(event Input|AxisEvents|InputAxisMoveRight
  (params (AxisValue :type Float%20%28single-precision%29))
  (Pawn|Input|AddMovementInput (Game|Player|GetPlayerPawn 0) (Transformation|GetActorRightVector) AxisValue false))

(event Input|AxisEvents|InputAxisTurn
  (params (AxisValue :type Float%20%28single-precision%29))
  (Pawn|Input|AddControllerYawInput (Game|Player|GetPlayerPawn 0) AxisValue))

(event Input|AxisEvents|InputAxisLookUp
  (params (AxisValue :type Float%20%28single-precision%29))
  (Pawn|Input|AddControllerPitchInput (Game|Player|GetPlayerPawn 0) AxisValue))

(fn ConstructionScript)