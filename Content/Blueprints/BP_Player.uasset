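; Player shooter Blueprint that manages ammo, health, walk speed and hitscan firing at BP_Monster targets.
; Fire spends ammo, plays a montage, traces from screen centre, then traces from the gun socket using that hit to pick the monster to damage.
; Ammo and health changes call notify events; R refills ammo.
; Death only prints a message, and HealHealth sets Health to max whenever the healed value is at or below max.
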(event Input|KeyboardEvents|R
  (params (Key :type Key%20Structure :default "None"))
  (:Pressed
    (Variables|Default|SetAmmoCount (Variables|Default|GetMaxAmmo))
    (Default|CallOnAmmoChange)))

(fn ConstructionScript
  (Variables|Default|SetAmmoCount (Variables|Default|GetMaxAmmo))
  (Variables|Default|SetHealth (Variables|Default|GetMaxHealth)))

(fn Fire
  (if (> (Variables|Default|GetAmmoCount) 0)
    (bind _result (Math|Integer|DecrementInt (Variables|Default|GetAmmoCount))
      (:%20%20
        (Variables|Default|SetAmmoCount _result)
        (Utilities|FlowControl|Sequence
          (:then_0
            (Animation|PlayAnimMontage "/Game/Animations/AM_Fire.AM_Fire" 1.0 "Default")
            (bind _outhit (|AimScreenToTarget))
            (bind _asbp_monster (|AimPlayerToTarget 0 _outhit))
            (Default|TakeDamage _asbp_monster (Variables|Default|GetDamage)))
          (:then_1
            ;[0.15 0.15 0.15 0.5] 총 쏠때 이벤트를 호출
            (Default|CallOnAmmoChange)))))))

(fn TakeDamage
  (params (DamageIncome :type Integer))
  (bind _output_get (Variables|Default|SetHealth (- (Variables|Default|GetHealth) DamageIncome)))
  (Default|CallOnHealthChange)
  (if (<= _output_get 0)
    (Development|PrintString "죽었다잇")))

(fn MoveSlower
  (params (bIsSlower :type Boolean))
  (if bIsSlower
    (Variables|/Script/Engine.CharacterMovementComponent|SetMaxWalkSpeed (Variables|Character|GetCharacterMovement) 3e+02)
    (else
      (Variables|/Script/Engine.CharacterMovementComponent|SetMaxWalkSpeed (Variables|Character|GetCharacterMovement) 6e+02))))

(fn HealHealth
  (params (HealAmount :type Integer))
  (Utilities|FlowControl|Sequence
    (:then_0
      (bind _output_get (Variables|Default|SetHealth (+ HealAmount (Variables|Default|GetHealth))))
      (if (<= _output_get (Variables|Default|GetMaxHealth))
        (Variables|Default|SetHealth (Variables|Default|GetMaxHealth))))
    (:then_1
      (Default|CallOnHealthChange))))