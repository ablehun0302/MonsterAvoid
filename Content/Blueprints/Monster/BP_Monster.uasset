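; BP_Monster is an enemy monster with health and a montage-based attack.
; Attack plays the monster attack montage, while the logic that would damage the player character is disconnected and never runs.
; TakeDamage subtracts incoming damage from Health, destroying the actor at zero or below and otherwise printing the remaining health.
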(fn ConstructionScript)

(fn Attack
  (Animation|PlayAnimMontage "/Game/Animations/AM_MonsterAttack.AM_MonsterAttack" 1.0 "Attack"))

(fn TakeDamage
  (params (DamageIncome :type Integer))
  (bind _output_get (Variables|Default|SetHealth (- (Variables|Default|GetHealth) DamageIncome)))
  (if (<= _output_get 0)
    (Actor|DestroyActor)
    (else
      (Development|PrintString (Utilities|String|ToString(Integer) (Variables|Default|GetHealth))))))