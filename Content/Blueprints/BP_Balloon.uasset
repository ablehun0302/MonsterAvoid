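; BP_Balloon is an actor that floats upward and removes itself once it climbs high enough.
; BeginPlay picks a random rise speed for each instance.
; Tick moves the actor along its local Z axis by that speed scaled by delta time, then destroys it when its world Z reaches MaxHeight.
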(event EventTick
  (params (DeltaSeconds :type Float%20%28single-precision%29))
  (Transformation|AddActorLocalOffset (Math|Vector|MakeVector 0.0 0.0 (* DeltaSeconds (Variables|Default|GetRiseSpeed))) false false)
  (if (>= (.z (Transformation|GetActorLocation)) (Variables|Default|GetMaxHeight))
    (Actor|DestroyActor)))

(event EventBeginPlay
  (Variables|Default|SetRiseSpeed (Math|Random|RandomFloatinRange 5e+01 2e+02)))

(fn ConstructionScript)