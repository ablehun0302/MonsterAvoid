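; Game mode for a timed monster-hunting round that keeps the level stocked with monsters until time runs out.
; BeginPlay caches the player and spawns the maximum monster count at random reachable points around WorldCenter.
; Tick refills one at a time via a DoOnce-gated random delay, prints health and time, then destroys all monsters at the limit.
; SetMonsterKillAmount increments and prints the kill count.
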(event EventBeginPlay
  ;[0.15 0.15 0.15 0.5] 플레이어 가져오기
  (bind _asbp_player (Utilities|Casting|CastToBP_Player (Game|Player|GetPlayerPawn 0))
    (:then
      (Variables|Default|SetPlayer _asbp_player)
      ;[0.15 0.15 0.15 0.5] 시작 시 몬스터 생성
      (for _index (range 1 (Variables|Default|GetMaxMonsterAmount))
        (CallFunction|SpawnMonster)))
    (:CastFailed
      (Development|PrintString "플레이어 없슈" true true "(R=1.000000,G=0.091247,B=0.000000,A=1.000000)" 1e+01))))

(event EventTick
  (params (DeltaSeconds :type Float%20%28single-precision%29))
  (Utilities|FlowControl|Sequence
    (:then_0
      ;[0.15 0.15 0.15 0.5] 적 10마리 미만일때 추가 생성 로직
      (if (Variables|Default|GetbIsPlaying)
        (bind _outactors (Actor|GetAllActorsOfClass "/Game/Blueprints/Monster/BP_Monster.BP_Monster_C"))
        (if (< (Utilities|Array|Length _outactors) (Variables|Default|GetMaxMonsterAmount))
          (Utilities|FlowControl|DoOnce false :!label _label
            (:Completed
              (Utilities|FlowControl|Delay (Math|Random|RandomFloatinRange 1.0 5.0))
              (CallFunction|SpawnMonster)
              (goto _label Reset))))))
    (:then_1
      (if (<= (+ (Utilities|Time|GetWorldDeltaSeconds) (Variables|Default|GetCurrentTime)) (Variables|Default|GetLimitTime))
        (Variables|Default|SetCurrentTime (+ (Utilities|Time|GetWorldDeltaSeconds) (Variables|Default|GetCurrentTime)))
        (CallFunction|PrintLog)
        (else
          (Utilities|FlowControl|DoOnce false
            (:Completed
              (Variables|Default|SetbIsPlaying false)
              (Development|PrintString "게임 끝!" true true "(R=1.000000,G=0.862207,B=0.000000,A=1.000000)" 1e+02)
              (bind _outactors_2 (Actor|GetAllActorsOfClass "/Game/Blueprints/Monster/BP_Monster.BP_Monster_C"))
              (for _array_element _outactors_2
                (Actor|DestroyActor _array_element)))))))))

(fn ConstructionScript)

(fn SpawnMonster
  (Game|SpawnActorfromClass "/Game/Blueprints/Monster/BP_Monster.BP_Monster_C" (Math|Transform|MakeTransform (.RandomLocation (AI|Navigation|GetRandomReachablePointinRadius (Variables|Default|GetWorldCenter) (Variables|Default|GetSpawnRadius) 0 0)) "0, 0, 0" "1.000000,1.000000,1.000000") "Undefined" "MultiplyWithRoot" 0 0))

(fn SetMonsterKillAmount
  (bind _result (Math|Integer|IncrementInt (Variables|Default|GetMonsterKillAmount))
    (:%20%20
      (Variables|Default|SetMonsterKillAmount _result)
      (Development|PrintText (Utilities|Text|FormatText "처치한 몬스터: {0} 마리" (Variables|Default|GetMonsterKillAmount))))))

(fn PrintLog
  (Development|PrintText (Utilities|Text|FormatText "플레이어 체력: {0}" (Variables|/Game/Blueprints/BP_Player.BP_Player_C|GetHealth (Variables|Default|GetPlayer))) true true "(R=0.000000,G=0.660000,B=1.000000,A=1.000000)" 0.0)
  (Development|PrintText (Utilities|Text|FormatText "현재 시간: {0} , 제한 시간: {1}" (Class|KismetMathLibrary|ToInt64(Float) (Variables|Default|GetCurrentTime)) (Variables|Default|GetLimitTime)) true true "(R=0.000000,G=0.660000,B=1.000000,A=1.000000)" 0.0))