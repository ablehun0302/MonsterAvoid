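; BP_BounceTrap is a trap that knocks the player away and damages them on contact.
; When its Sphere component registers a hit with a BP_Player, it builds a random, upward-biased direction and scales it to BounceRange.
; It launches the character with that vector, adding to current velocity rather than overriding it, then calls TakeDamage on the player with its Damage value.
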(event OnComponentHit(Sphere)
  (params (HitComponent :type Primitive%20Component%20Object%20Reference) (OtherActor :type Actor%20Object%20Reference) (OtherComp :type Primitive%20Component%20Object%20Reference) (NormalImpulse :type Vector :default "0, 0, 0") (Hit :type Hit%20Result%20Structure%20%28by%20ref%29))
  (bind _bouncerange (Variables|Default|GetBounceRange))
  (bind _bouncerange_2 (Variables|Default|GetBounceRange))
  (bind _returnvalue (* _bouncerange_2 -1.0))
  (bind _asbp_player (Utilities|Casting|CastToBP_Player OtherActor))
  (bind _output_get (Variables|Default|SetRandomLocation (Math|Vector|MakeVector (Math|Random|RandomFloatinRange _returnvalue _bouncerange) (Math|Random|RandomFloatinRange _returnvalue _bouncerange) (Variables|Default|GetBounceRange))))
  (Character|LaunchCharacter _asbp_player (* (Math|Vector|Normalize _output_get) (Variables|Default|GetBounceRange)) false false)
  (Default|TakeDamage _asbp_player (Variables|Default|GetDamage)))

(fn ConstructionScript)