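; BP_Cannon is a trap that automatically fires cannonballs along its forward direction at a fixed interval.
; A countdown set from ShootInterval at BeginPlay decreases each Tick and resets after every shot.
; Each shot spawns a BP_Bullet just ahead of the cannon, ignoring collision, and applies an impulse scaled by CannonPower to its Cannonball component.
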(event EventTick
  (params (DeltaSeconds :type Float%20%28single-precision%29))
  (bind _output_get (Variables|Default|SetTime (- (Variables|Default|GetTime) DeltaSeconds)))
  (if (<= _output_get 0.0)
    (bind _returnvalue (Game|SpawnActorfromClass "/Game/Blueprints/Traps/BP_Bullet.BP_Bullet_C" (Math|Transform|MakeTransform (+ (Transformation|GetActorLocation) (* 1.9e+02 (Transformation|GetActorForwardVector))) (Transformation|GetActorRotation) "1.000000,1.000000,1.000000") "AlwaysSpawn" "MultiplyWithRoot" 0 0))
    (Physics|AddImpulse (Variables|/Game/Blueprints/Traps/BP_Bullet.BP_Bullet_C|Getcannonball _returnvalue) (* (Transformation|GetActorForwardVector) (Variables|Default|GetCannonPower)) "None" false)
    (Variables|Default|SetTime (Variables|Default|GetShootInterval))))

(event EventBeginPlay
  (Variables|Default|SetTime (Variables|Default|GetShootInterval)))

(fn ConstructionScript)